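; Game instance that manages the loading screen shown around level changes.
; LoadLevel creates a LoadScreen widget, hands it the target level name, stores it, adds it to the viewport and calls Fade(true).
; LoadedLevel re-adds the stored widget to the viewport if still valid, waits briefly, calls Fade(false) and clears the reference.
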(event Custom|LoadLevel
  (params (LevelName :type Name))
  (bind _returnvalue (UserInterface|CreateWidget "/Game/UI/LoadScreen.LoadScreen_C" (Game|GetPlayerController 0) LevelName))
  (bind _output_get (Variables|Default|SetW_LoadScreen _returnvalue))
  (UserInterface|Viewport|AddtoViewport _output_get 0)
  (Default|Fade (Variables|Default|GetW_LoadScreen) true))

(event Custom|LoadedLevel
  (bind _w_loadscreen (Variables|Default|GetW_LoadScreen)
    (:then
      (UserInterface|Viewport|AddtoViewport _w_loadscreen 0)
      (Utilities|FlowControl|Delay 2.0)
      (Default|Fade (Variables|Default|GetW_LoadScreen) false)
      (Variables|Default|SetW_LoadScreen 0))
    (:else)))