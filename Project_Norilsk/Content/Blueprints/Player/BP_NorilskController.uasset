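; Player controller for Norilsk that toggles a pause menu with Escape or Q.
; PauseMenu creates or removes the menu widget and sets the game's paused state to match, using the widget reference's validity as the toggle state.
; UIControl switches between Game-and-UI and game-only input, showing the cursor and disabling pawn input while the menu is open.
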(event Input|KeyboardEvents|Escape
  (params (Key :type Key%20Structure))
  (:Pressed
    (Variables|Default|GetW_PauseMenu
      (:then
        (CallFunction|PauseMenu false))
      (:else
        (CallFunction|PauseMenu true)))))

(event Input|KeyboardEvents|Q
  (params (Key :type Key%20Structure))
  (:Pressed
    (Variables|Default|GetW_PauseMenu
      (:then
        (CallFunction|PauseMenu false))
      (:else
        (CallFunction|PauseMenu true)))))

(fn ConstructionScript)

(fn PauseMenu
  (params (Show :type Boolean))
  (if Show
    (bind _returnvalue (UserInterface|CreateWidget "/Game/UI/PauseMenu.PauseMenu_C" self))
    (bind _output_get (Variables|Default|SetW_PauseMenu _returnvalue))
    (UserInterface|Viewport|AddtoViewport _output_get 0)
    (CallFunction|UIControl true (Variables|Default|GetW_PauseMenu))
    (Game|SetGamePaused true)
    (else
      (Utilities|IsValid (Variables|Default|GetW_PauseMenu)
        (:Is%20Valid
          (Widget|RemovefromParent (Variables|Default|GetW_PauseMenu))
          (Variables|Default|SetW_PauseMenu 0)
          (CallFunction|UIControl false)
          (Game|SetGamePaused false))))))

(fn UIControl
  (params (Activate :type Boolean) (WidgetToFocus :type Widget%20Object%20Reference))
  (bind _self self)
  (if Activate
    (Variables|Default|SetbShowMouseCursor true)
    (Input|SetInputModeGameandUI self WidgetToFocus "DoNotLock" true)
    (Input|DisableInput (Pawn|GetControlledPawn) self)
    (else
      (Variables|Default|SetbShowMouseCursor false)
      (Input|EnableInput (Pawn|GetControlledPawn) _self)
      (Input|SetInputModeGameOnly _self))))