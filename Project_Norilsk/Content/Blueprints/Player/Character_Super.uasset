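; Player character Blueprint that identifies itself with the "PlayerSuper" character row and starts with an unarmed weapon loadout.
; The construction script sets that row name after the parent's construction logic runs.
; On BeginPlay it runs the parent logic, adds "UnArmed" to the weapon inventory, and pads the name array with empty slots up to the inventory size.
; It then makes the first slot the active weapon.
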(event EventBeginPlay
  (|CallParentFunction)
  (CallFunction|AddtoWeaponInventory "UnArmed")
  (if (< (Utilities|Array|Length (Variables|Default|GetWeaponInvNames)) (Variables|Default|GetWpnInvSize)) :!label _label
    (Utilities|Array|SetArrayElem (Variables|Default|GetWeaponInvNames) (Utilities|Array|Length (Variables|Default|GetWeaponInvNames)) "" true)
    (goto _label)
    (else
      (CallFunction|SetActiveWpnVars))))

(event Collision|EventActorBeginOverlap
  (params (OtherActor :type Actor%20Object%20Reference)))

(event EventTick
  (params (DeltaSeconds :type Float%20%28single-precision%29)))

(fn ConstructionScript
  (|CallParentFunction)
  (Variables|Default|SetCharRowName "PlayerSuper"))